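; Actor Blueprint that moves its Cube around a square path in a continuous loop while spinning it.
; Each Tick adds a fixed relative offset and world rotation, so speed depends on frame rate.
; Three boolean flags select the leg: +X and +Y out to Endpoint, then -X and -Y back to zero.
; All three flags reset when the last leg finishes, restarting the loop.
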(event EventTick
  (params (DeltaSeconds :type Float%20%28single-precision%29))
  (bind _cube (Variables|Default|GetCube))
  (bind _cube_2 (Variables|Default|GetCube))
  (bind _cube_3 (Variables|Default|GetCube))
  (bind _cube_4 (Variables|Default|GetCube))
  (if (Variables|Default|GetIsMoveRit1)
    (Transformation|AddRelativeLocation _cube_4 "10.000000, 0,0.000000" false false)
    (Transformation|AddWorldRotation (Variables|Default|GetCube) "0.000000,10.000000,0.000000" false false)
    (if (>= (.x (Variables|/Script/Engine.SceneComponent|GetRelativeLocation _cube_4)) (Variables|Default|GetEndpoint))
      (Variables|Default|SetIsMoveRit1 false))
    (elif (Variables|Default|GetIsMoveRit2)
      (Transformation|AddRelativeLocation _cube "0.000000,10.000000,0.000000" false false)
      (Transformation|AddWorldRotation (Variables|Default|GetCube) "0.000000,10.000000,0.000000" false false)
      (if (>= (.y (Variables|/Script/Engine.SceneComponent|GetRelativeLocation _cube)) (Variables|Default|GetEndpoint))
        (Variables|Default|SetIsMoveRit2 false))
      (elif (Variables|Default|GetIsMoveRit3)
        (Transformation|AddRelativeLocation _cube_2 "-10.000000, 0,0.000000" false false)
        (Transformation|AddWorldRotation (Variables|Default|GetCube) "0.000000,10.000000,0.000000" false false)
        (if (<= (.x (Variables|/Script/Engine.SceneComponent|GetRelativeLocation _cube_2)) 0.0)
          (Variables|Default|SetIsMoveRit3 false))
        (else
          (Transformation|AddRelativeLocation _cube_3 "0.000000,-10.000000,0.000000" false false)
          (Transformation|AddWorldRotation (Variables|Default|GetCube) "0.000000,10.000000,0.000000" false false)
          (if (<= (.y (Variables|/Script/Engine.SceneComponent|GetRelativeLocation _cube_3)) 0.0)
            (Variables|Default|SetIsMoveRit1 true)
            (Variables|Default|SetIsMoveRit2 true)
            (Variables|Default|SetIsMoveRit3 true)))))))

(fn ConstructionScript)