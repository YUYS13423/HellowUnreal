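; Movement test actor that moves a Cube by relative offsets according to a direction enum, EnMove, starting at BeginPlay.
; Right, Up and Left drive timeline 1 into 이동x (X plus constant Y drift); Down drives timeline 2 into 이동y.
; On finish, RL변환 or UD변환 updates the direction and the switch re-runs, though Up stays unchanged through RL변환.
; An unfinished curved-path timeline is left unconnected.
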(event EventBeginPlay
  (bind _en_move (Variables|Default|GetEn%20Move))
  (bind _속도 (Variables|Default|Get속도))
  (switch Utilities|FlowControl|Switch|SwitchonEn_Move_Tipe (Variables|Default|GetEn%20Move) :!label _label
    (:NewEnumerator0
      (Variables|Default|Set방향전환 1.0)
      (bind _새_트랙_0 (Timeline|1 Play)
        (:Update
          (CallFunction|이동x _새_트랙_0 _속도 (Variables|Default|Get방향전환)))
        (:Finished
          (CallFunction|RL변환 _en_move)
          (goto _label))))
    (:NewEnumerator1
      (Variables|Default|Set방향전환 1.0)
      (Timeline|1 Reverse))
    (:NewEnumerator2
      (Variables|Default|Set방향전환 -1.0)
      (Timeline|1 Reverse))
    (:NewEnumerator3
      (Variables|Default|Set방향전환 -1.0)
      (bind _새_트랙_0_2 (Timeline|2 Reverse)
        (:Update
          (CallFunction|이동y _새_트랙_0_2 _속도 (Variables|Default|Get방향전환)))
        (:Finished
          (CallFunction|UD변환 _en_move)
          (goto _label))))))

(fn ConstructionScript)

(fn 이동x
  (params (B :type Float%20%28single-precision%29) (NewParam :type Float%20%28single-precision%29) (NewParam1 :type Float%20%28single-precision%29))
  (Transformation|AddRelativeLocation (Variables|Default|GetCube) (Math|Vector|MakeVector (* NewParam B NewParam1) 1e+01 0.0) false false)
  (Development|PrintString "x"))

(fn 이동y
  (params (B :type Float%20%28single-precision%29) (NewParam :type Float%20%28single-precision%29) (NewParam1 :type Float%20%28single-precision%29))
  (Transformation|AddRelativeLocation (Variables|Default|GetCube) (Math|Vector|MakeVector 0.0 (* NewParam B NewParam1) 0.0) false false)
  (Development|PrintString "y"))

(fn UD변환
  (params (NewParam :type En_Move_Tipe%20Enum :default "NewEnumerator0"))
  (if (Utilities|Enum|Equal(Enum) NewParam "NewEnumerator1")
    (Variables|Default|SetEn%20Move "NewEnumerator2")
    (return)
    (elif (Utilities|Enum|Equal(Enum) NewParam "NewEnumerator3")
      (Variables|Default|SetEn%20Move "NewEnumerator0")
      (return))))

(fn RL변환
  (params (NewParam :type En_Move_Tipe%20Enum :default "NewEnumerator0"))
  (if (Utilities|Enum|Equal(Enum) NewParam "NewEnumerator0")
    (Variables|Default|SetEn%20Move "NewEnumerator1")
    (return)
    (elif (Utilities|Enum|Equal(Enum) NewParam "NewEnumerator2")
      (Variables|Default|SetEn%20Move "NewEnumerator3")
      (return))))